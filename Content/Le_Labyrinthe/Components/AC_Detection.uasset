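; AC_Detection is a component that detects BP_Torche actors by line trace when IA_LineTrace triggers.
; The debug-drawn CastLine trace starts at the owner's XY position with Z fixed at one.
; Its end adds the product of the control-rotation forward vector's X and Y, not a scaled direction.
; Hits print the actor's name, and a blocking torch hit calls SetActive false on the component itself.
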(event Input|EnhancedActionEvents|EnhancedInputActionIA_LineTrace
  (params (ActionValue :type Boolean) (ElapsedSeconds :type Float%20%28double-precision%29) (TriggeredSeconds :type Float%20%28double-precision%29) (InputAction :type Input%20Action%20Object%20Reference :default "/Game/Le_Labyrinthe/Inputs/InputAction/IA_LineTrace.IA_LineTrace"))
  (bind _returnvalue (Game|GetPlayerController 0))
  (bind _returnvalue_2 (Components|GetOwner))
  (bind _returnvalue_3 (Pawn|GetControlRotation _returnvalue :!class /Script/Engine.Controller))
  (bind _returnvalue_4 (Transformation|GetActorLocation _returnvalue_2))
  (bind (_x _y) (Class|KismetMathLibrary|BreakVector3f _returnvalue_4))
  (bind (_x_2 _y_2) (Class|KismetMathLibrary|BreakVector3f _returnvalue_4))
  (bind _returnvalue_5 (Math|Vector|GetForwardVector _returnvalue_3))
  (:Triggered
    (bind _output_get (Variables|Default|SetStartLineTrace (Math|Vector|MakeVector _x_2 _y_2 1.0)))
    (bind _output_get_2 (Variables|Default|SetEndLineTrace (+ (Math|Vector|MakeVector _x _y 1.0) (* (.x _returnvalue_5) (.y _returnvalue_5)))))
    (if true
      (bind (_outhit _returnvalue_6) (Collision|LineTraceByChannel _output_get _output_get_2 (Variables|Default|GetCastLine) false 0 "ForDuration"))
      (if _returnvalue_6
        (Development|PrintString (Utilities|GetDisplayName (.HitActor (Collision|BreakHitResult _outhit))))
        (Utilities|Casting|CastToBP_Torche (.HitActor (Collision|BreakHitResult _outhit)))
        (if (.bBlockingHit (Collision|BreakHitResult _outhit))
          (Components|Activation|SetActive false false))))))