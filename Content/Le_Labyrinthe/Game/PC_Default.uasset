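; PC_Default is the player controller that routes Enhanced Input to the first-person character, BP_FirstPersonCharacter.
; On BeginPlay it adds the IMC_Character mapping context.
; IA_Move moves the character along axes derived from control rotation, and IA_Mouse adds yaw and pitch to the controller.
; IA_LineTrace only looks up the character and performs no trace here.
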(event Input|EnhancedActionEvents|EnhancedInputActionIA_Move
  (params (ActionValue :type Vector%202D%20Structure) (ElapsedSeconds :type Float%20%28double-precision%29) (TriggeredSeconds :type Float%20%28double-precision%29) (InputAction :type Input%20Action%20Object%20Reference :default "/Game/Le_Labyrinthe/Inputs/InputAction/IA_Move.IA_Move"))
  (bind _returnvalue (Pawn|GetControlRotation :!class /Script/Engine.Controller))
  ;[1 1 1] Movement
  ;;[1 1 1] Player Movement
  (:Triggered
    (bind _returnvalue_2 (Actor|GetActorOfClass "/Game/Le_Labyrinthe/Blueprints/BP_FirstPersonCharacter.BP_FirstPersonCharacter_C"))
    (Pawn|Input|AddMovementInput _returnvalue_2 (Math|Vector|GetRightVector (Math|Rotator|MakeRotator (.roll _returnvalue) 0.0 (.yaw _returnvalue))) (.x ActionValue) false)
    (Pawn|Input|AddMovementInput _returnvalue_2 (Math|Vector|GetForwardVector (Math|Rotator|MakeRotator 0.0 0.0 (.yaw _returnvalue))) (.y ActionValue) false)))

(event Input|EnhancedActionEvents|EnhancedInputActionIA_Mouse
  (params (ActionValue :type Vector%202D%20Structure) (ElapsedSeconds :type Float%20%28double-precision%29) (TriggeredSeconds :type Float%20%28double-precision%29) (InputAction :type Input%20Action%20Object%20Reference :default "/Game/Le_Labyrinthe/Inputs/InputAction/IA_Mouse.IA_Mouse"))
  ;[1 1 1] Movement
  ;;[1 1 1] Mouse Movement
  (:Triggered
    (Class|PlayerController|AddYawInput (.x ActionValue))
    (Class|PlayerController|AddPitchInput (.y ActionValue))))

(event Input|EnhancedActionEvents|EnhancedInputActionIA_LineTrace
  (params (ActionValue :type Boolean) (ElapsedSeconds :type Float%20%28double-precision%29) (TriggeredSeconds :type Float%20%28double-precision%29) (InputAction :type Input%20Action%20Object%20Reference :default "/Game/Le_Labyrinthe/Inputs/InputAction/IA_LineTrace.IA_LineTrace"))
  ;[1 1 1] LineTrace
  (:Started
    (Actor|GetActorOfClass "/Game/Le_Labyrinthe/Blueprints/BP_FirstPersonCharacter.BP_FirstPersonCharacter_C")))

(event EventBeginPlay
  (bind _self self)
  (bind _returnvalue (PlayerController|LocalPlayerSubsystems|GetEnhancedInputLocalPlayerSubsystem _self))
  ;[1 1 1] Set mapping context
  (Utilities|IsValid _returnvalue
    (:Is%20Valid
      (Input|AddMappingContext _returnvalue "/Game/Le_Labyrinthe/Inputs/InputMapping/IMC_Character.IMC_Character" 0 "(bIgnoreAllPressedKeysUntilRelease=True,bForceImmediately=False)")
      (Utilities|Casting|CastToBP_FirstPersonCharacter (Game|GetPlayerCharacter 0)))))

(fn ConstructionScript)